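; Controller for the main menu of a match-3 RPG that manages stage selection and progression.
; ShowMainMenu creates the BP_MainMenu widget with the stage list, current stage, player and shop, then adds it to the viewport.
; The menu's battle click is relayed through the OnStageSelected dispatcher with the chosen stage data.
; OnStageCleared advances the current stage, clamped between zero and the stage list's length.
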(event `ShowMainMenu`
  (params (player :type "/Game/Match3RPGTemplate/Blueprints/Units/BP_UnitBase Class Reference") (shop :type "/Game/Match3RPGTemplate/Blueprints/BP_Shop Object Reference"))
  ;[1 1 1] Creates the main and shows it
  (bind _returnvalue (`|CreateWidget` "/Game/Match3RPGTemplate/Blueprints/UI/MainMenu/BP_MainMenu.BP_MainMenu_C" null (`self.listOfStages`) (`self.currentStage`) player shop))
  (bind _output_get (set `self.mainMenu` _returnvalue))
  (`UserWidget.AddToViewport` _output_get 0)
  (add `/Game/Match3RPGTemplate/Blueprints/UI/MainMenu/BP_MainMenu.OnBattleClicked` (`self.mainMenu`) (delegate `OnBattleClickedHandler`)))

(event `OnBattleClickedHandler`
  (params (stageData :type "/Game/Match3RPGTemplate/Blueprints/StageData Structure"))
  ;[1 1 1] Creates the main and shows it
  (`self.OnStageSelected` stageData))

(event `OnStageCleared`
  ;[1 1 1] Sets the current stage
  (set `self.currentStage` (`KismetMathLibrary.Clamp` (+ (`self.currentStage`) 1) 0 (`KismetArrayLibrary.Array_Length` (`self.listOfStages`)))))

(fn `UserConstructionScript`)