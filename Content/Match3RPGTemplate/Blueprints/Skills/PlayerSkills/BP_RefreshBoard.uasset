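; BP_RefreshBoard is a player skill in the Match-3 RPG template that destroys all gems on the board and creates new ones.
; On use, it binds a handler to the board's rearranged event through the battle manager's game UI, then triggers the refresh.
; When the board finishes rearranging, the handler unbinds itself and signals that the skill was used, so completion waits on the board.
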(event `self.UseSkill`
  (bind _board (`/Game/Match3RPGTemplate/Blueprints/UI/BP_GameUI.Board` (`/Game/Match3RPGTemplate/Blueprints/BP_Match3RPGPlayerController.GameUI` (`/Game/Match3RPGTemplate/Blueprints/BP_BattleManager.match3RPGPlayerController` (`self.battleManager`)))))
  ;[1 1 1] Destroy all gems and create new ones
  (add `/Game/Match3RPGTemplate/Blueprints/UI/BP_Board.OnBoardReArranged` _board (delegate `OnBoardReArrangedHandler`))
  (`/Game/Match3RPGTemplate/Blueprints/UI/BP_Board.RefreshBoard` _board))

(event `OnBoardReArrangedHandler`
  ;[1 1 1] Destroy all gems and create new ones
  (remove `/Game/Match3RPGTemplate/Blueprints/UI/BP_Board.OnBoardReArranged` (`/Game/Match3RPGTemplate/Blueprints/UI/BP_GameUI.Board` (`/Game/Match3RPGTemplate/Blueprints/BP_Match3RPGPlayerController.GameUI` (`/Game/Match3RPGTemplate/Blueprints/BP_BattleManager.match3RPGPlayerController` (`self.battleManager`)))) (delegate `OnBoardReArrangedHandler`))
  (`self.OnSkillUsed`))

(fn `UserConstructionScript`
  (`parent.UserConstructionScript`))