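; Base Blueprint for player skills in the Match-3 RPG template, tracking a skill's turn-based cooldown and destroying itself when the BattleManager's player unit is destroyed.
; Using the skill resets the cooldown to one above its configured value, and the per-turn reduction clamps it between zero and that value.
; Each reduction refreshes the linked skill button UI, which is assigned through a setter event.
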(event `self.ReceiveBeginPlay`
  ;[1 1 1] Destroy when player unit is destroyed
  (add `self.OnDestroyed` (`/Game/Match3RPGTemplate/Blueprints/BP_BattleManager.player` (`self.battleManager`)) (delegate `OnPlayerDestroyed`)))

(event `OnPlayerDestroyed` :!signature `self.OnDestroyed`
  (params (DestroyedActor :type "Actor Object Reference"))
  ;[1 1 1] Destroy when player unit is destroyed
  (`self.K2_DestroyActor`))

(event `SetSkillButtonUI`
  (params (skillButtonUI :type "/Game/Match3RPGTemplate/Blueprints/UI/Skills/BP_SkillButton Object Reference"))
  ;[1 1 1] Set button
  (set `self.skillButtonUI` skillButtonUI))

(event `ResetCooldown`
  ;[1 1 1] Reset cooldown after using skill
  (set `self.currentCooldown` (+ (`self.cooldown`) 1)))

(event `ReduceCooldown`
  ;[1 1 1] Reduce cooldown after every turn
  (set `self.currentCooldown` (`KismetMathLibrary.Clamp` (- (`self.currentCooldown`) 1) 0 (`self.cooldown`)))
  (`/Game/Match3RPGTemplate/Blueprints/UI/Skills/BP_SkillButton.UpdateCooldown` (`self.skillButtonUI`)))

(fn `UserConstructionScript`
  (`parent.UserConstructionScript`))