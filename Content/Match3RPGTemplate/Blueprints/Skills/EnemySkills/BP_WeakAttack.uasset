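; BP_WeakAttack is an enemy skill in the Match-3 RPG template that performs a basic melee attack on the player.
; UseSkill moves the enemy to the player, plays its attack animation and triggers BattleManager damage at the animation's hit delay.
; After the remaining animation time it moves the enemy back, chaining steps through completion handlers, then signals that the skill was used.
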(event `self.UseSkill`
  ;[1 1 1] Move enemy next to player
  (`self.EnemyMove` (delegate `OnMovedToPlayerHandler`)))

(event `OnMovedToPlayerHandler`
  ;[1 1 1] Move enemy next to player
  (`self.PlayAttack`))

(event `PlayAttack`
  (bind _currentenemy (`/Game/Match3RPGTemplate/Blueprints/BP_BattleManager.currentEnemy` (`self.battleManager`)))
  (bind _animationhitdelay (`/Game/Match3RPGTemplate/Blueprints/Units/BP_UnitBase.animationHitDelay` _currentenemy))
  ;[1 1 1] Enemy unit attacks
  (bind _animationlength (`/Game/Match3RPGTemplate/Blueprints/Units/BP_UnitBase.PlayAnimation` _currentenemy "NewEnumerator3"))
  (`KismetSystemLibrary.Delay` _animationhitdelay)
  (`/Game/Match3RPGTemplate/Blueprints/BP_BattleManager.EnemyDoDamage` (`self.battleManager`))
  (bind _returnvalue (- _animationlength _animationhitdelay))
  (`KismetSystemLibrary.Delay` (select `bool` (> _returnvalue 0.0) :`true` _returnvalue))
  (`self.EnemyMoveBack` (delegate `OnEnemyMovedBackHandler`)))

(event `OnEnemyMovedBackHandler`
  ;[1 1 1] Enemy unit attacks
  (`self.OnSkillUsed`))

(fn `UserConstructionScript`
  (`parent.UserConstructionScript`))