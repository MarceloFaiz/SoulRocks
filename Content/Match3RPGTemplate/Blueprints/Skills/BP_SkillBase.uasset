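; Base skill Blueprint for Match3 RPG battles, with an empty UseSkill event that child classes override.
; Provides shared helpers to hide or show the game UI through the player controller.
; Move helpers send the player or current enemy to the opponent's attack point, or back to its stage spawn at double speed.
; Each delegates to BattleManager's UnitMove, first binding the caller's callback to OnUnitMoved to signal movement completion.
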(event `UseSkill`
  ;[1 1 1] Override in child class
)

(event `HideUI`
  ;[1 1 1] Hide / show UI
  (bind _asbp_match_3rpgplayer_controller (cast `/Game/Match3RPGTemplate/Blueprints/BP_Match3RPGPlayerController` (`GameplayStatics.GetPlayerController` 0)))
  (bind _gameui (`/Game/Match3RPGTemplate/Blueprints/BP_Match3RPGPlayerController.GameUI` _asbp_match_3rpgplayer_controller))
  (`/Engine/EditorBlueprintResources/StandardMacros.IsValid` _gameui
    (:`Is Valid`
      (`/Game/Match3RPGTemplate/Blueprints/UI/BP_GameUI.HideUI` _gameui))))

(event `ShowUI`
  ;[1 1 1] Hide / show UI
  (bind _asbp_match_3rpgplayer_controller (cast `/Game/Match3RPGTemplate/Blueprints/BP_Match3RPGPlayerController` (`GameplayStatics.GetPlayerController` 0)))
  (bind _gameui (`/Game/Match3RPGTemplate/Blueprints/BP_Match3RPGPlayerController.GameUI` _asbp_match_3rpgplayer_controller))
  (`/Engine/EditorBlueprintResources/StandardMacros.IsValid` _gameui
    (:`Is Valid`
      (`/Game/Match3RPGTemplate/Blueprints/UI/BP_GameUI.ShowUI` _gameui))))

(fn `EnemyMove`
  (params (EnemyMove :type "Delegate (by ref)"))
  (bind _battlemanager (`self.battleManager`))
  (bind _currentenemy (`/Game/Match3RPGTemplate/Blueprints/BP_BattleManager.currentEnemy` _battlemanager))
  (`self.Move` EnemyMove "NewEnumerator1" (`/Game/Match3RPGTemplate/Blueprints/Units/BP_UnitBase.moveSpeed` _currentenemy) (`self.K2_GetActorLocation` _currentenemy) (`SceneComponent.K2_GetComponentLocation` (`/Game/Match3RPGTemplate/Blueprints/Units/BP_UnitBase.AttackLocation` (`/Game/Match3RPGTemplate/Blueprints/BP_BattleManager.player` _battlemanager))) (`/Game/Match3RPGTemplate/Blueprints/BP_BattleManager.currentEnemy` (`self.battleManager`))))

(fn `EnemyMoveBack`
  (params (EnemyMoveBack :type "Delegate (by ref)"))
  (bind _battlemanager (`self.battleManager`))
  (bind _currentenemy (`/Game/Match3RPGTemplate/Blueprints/BP_BattleManager.currentEnemy` _battlemanager))
  (`self.Move` EnemyMoveBack "NewEnumerator2" (* (`/Game/Match3RPGTemplate/Blueprints/Units/BP_UnitBase.moveSpeed` _currentenemy) 2.0) (`self.K2_GetActorLocation` _currentenemy) (`SceneComponent.K2_GetComponentLocation` (`/Game/Match3RPGTemplate/Blueprints/Stages/BP_StageBase.EnemySpawnLocation` (`/Game/Match3RPGTemplate/Blueprints/BP_BattleManager.stage` _battlemanager))) (`/Game/Match3RPGTemplate/Blueprints/BP_BattleManager.currentEnemy` (`self.battleManager`))))

(fn `Move`
  (params (Move :type "Delegate (by ref)") (moveAnimation :type "/Game/Match3RPGTemplate/Blueprints/Units/AnimationType Enum" :default "NewEnumerator0") (moveSpeed :type "Float (double-precision)") (fromLocation :type "Vector Structure") (toLocation :type "Vector Structure") (unit :type "/Game/Match3RPGTemplate/Blueprints/Units/BP_UnitBase Object Reference"))
  (add `/Game/Match3RPGTemplate/Blueprints/BP_BattleManager.OnUnitMoved` (`self.battleManager`) Move)
  (`/Game/Match3RPGTemplate/Blueprints/BP_BattleManager.UnitMove` (`self.battleManager`) moveAnimation moveSpeed fromLocation toLocation unit))

(fn `PlayerMove`
  (params (PlayerMove :type "Delegate (by ref)"))
  (bind _battlemanager (`self.battleManager`))
  (bind _player (`/Game/Match3RPGTemplate/Blueprints/BP_BattleManager.player` _battlemanager))
  (`self.Move` PlayerMove "NewEnumerator1" (`/Game/Match3RPGTemplate/Blueprints/Units/BP_UnitBase.moveSpeed` _player) (`self.K2_GetActorLocation` _player) (`SceneComponent.K2_GetComponentLocation` (`/Game/Match3RPGTemplate/Blueprints/Units/BP_UnitBase.AttackLocation` (`/Game/Match3RPGTemplate/Blueprints/BP_BattleManager.currentEnemy` _battlemanager))) (`/Game/Match3RPGTemplate/Blueprints/BP_BattleManager.player` (`self.battleManager`))))

(fn `PlayerMoveBack`
  (params (PlayerMoveBack :type "Delegate (by ref)"))
  (bind _battlemanager (`self.battleManager`))
  (bind _player (`/Game/Match3RPGTemplate/Blueprints/BP_BattleManager.player` _battlemanager))
  (`self.Move` PlayerMoveBack "NewEnumerator2" (* (`/Game/Match3RPGTemplate/Blueprints/Units/BP_UnitBase.moveSpeed` _player) 2.0) (`self.K2_GetActorLocation` _player) (`SceneComponent.K2_GetComponentLocation` (`/Game/Match3RPGTemplate/Blueprints/Stages/BP_StageBase.PlayerSpawnLocation` (`/Game/Match3RPGTemplate/Blueprints/BP_BattleManager.stage` _battlemanager))) (`/Game/Match3RPGTemplate/Blueprints/BP_BattleManager.player` (`self.battleManager`))))

(fn `UserConstructionScript`)