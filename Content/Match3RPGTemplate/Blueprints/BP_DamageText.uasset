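; BP_DamageText is a floating damage number actor that displays a Damage value in a given TextColor.
; On BeginPlay it gets the BP_DamageTextUI from its widget component and passes it the damage and color.
; It binds to the widget's Appear animation finishing, then unbinds and destroys itself when that animation ends.
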(event `self.ReceiveBeginPlay`
  ;[1 1 1] Set the damage
  (bind _output_get (set `self.damageTextUI` (cast `/Game/Match3RPGTemplate/Blueprints/UI/BP_DamageTextUI` (`WidgetComponent.GetUserWidgetObject` (`self.DamageTextUIWidget`)) :!pure true)))
  (`UserWidget.BindToAnimationFinished` _output_get (`/Game/Match3RPGTemplate/Blueprints/UI/BP_DamageTextUI.Appear` _output_get) (delegate `OnAnimationFinishedHandler`))
  (`/Game/Match3RPGTemplate/Blueprints/UI/BP_DamageTextUI.SetDamage` (`self.damageTextUI`) (`self.damage`) (`self.textColor`)))

(event `OnAnimationFinishedHandler`
  ;[1 1 1] Set the damage
  (`UserWidget.UnbindAllFromAnimationFinished` (`self.damageTextUI`) (`/Game/Match3RPGTemplate/Blueprints/UI/BP_DamageTextUI.Appear` (`self.damageTextUI`)))
  (`self.K2_DestroyActor`))

(fn `UserConstructionScript`)