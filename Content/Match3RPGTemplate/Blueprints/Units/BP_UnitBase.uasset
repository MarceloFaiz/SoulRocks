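; BP_UnitBase is the base actor for units in the Match 3 RPG template, handling spawning, health and animation.
; Spawn resets HP, plays idle and delegates placement to an optional spawn style actor, falling back to instant placement, then signals completion.
; Damage and healing route through a clamped HP setter that broadcasts updates.
; Animations play directly on the skeletal mesh by type, and Dissolve sinks the unit via timeline before destroying it.
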(event `Spawn`
  (params (spawnLocation :type "/Game/Match3RPGTemplate/Blueprints/BP_UnitSpawnLocation Object Reference"))
  ;[1 1 1] Spaw
  (`self.SetHP` (`self.maxHP`))
  (`self.PlayAnimation` "NewEnumerator0")
  (`self.InitializeSpawnStyle` spawnLocation))

(event `InitializeSpawnStyle`
  (params (spawnLocation :type "/Game/Match3RPGTemplate/Blueprints/BP_UnitSpawnLocation Object Reference"))
  ;[1 1 1] Create spawn style
  (if (`KismetSystemLibrary.IsValidClass` (`self.spawnStyleClass`))
    (bind _returnvalue (`|SpawnActorFromClass` (`self.spawnStyleClass`) (`KismetMathLibrary.MakeTransform` (0.0 0.0 0.0)) "Undefined" "OverrideRootScale" null self spawnLocation null))
    (add `/Game/Match3RPGTemplate/Blueprints/SpawnStyles/BP_SpawnStyleBase.OnSpawnFinished` _returnvalue (delegate `OnSpawnFinishedHandler`))
    (`/Game/Match3RPGTemplate/Blueprints/SpawnStyles/BP_SpawnStyleBase.Spawn` _returnvalue)
    (else
      (`self.DefaultSpawn` spawnLocation))))

(event `OnSpawnFinishedHandler`
  ;[1 1 1] Create spawn style
  (`self.OnUnitSpawned`))

(event `DefaultSpawn`
  (params (spawnLocation :type "/Game/Match3RPGTemplate/Blueprints/BP_UnitSpawnLocation Object Reference"))
  ;[1 1 1] Insta spawn the unit if no spawn style is given
  (`self.K2_SetActorTransform` (`self.GetTransform` spawnLocation))
  (`self.OnUnitSpawned`))

(event `TakeDamage`
  (params (damage :type Integer))
  ;[1 1 1] Deduct Hp
  (`self.SetHP` (- (`self.currentHP`) damage)))

(event `Heal`
  (params (healAmount :type Integer))
  ;[1 1 1] Add Hp
  (`self.SetHP` (+ healAmount (`self.currentHP`))))

(event `SetHP`
  (params (hp :type Integer))
  ;[1 1 1] Set Hp
  (set `self.currentHP` (`KismetMathLibrary.Clamp` hp 0 (`self.maxHP`)))
  (`self.OnHPUpdated`))

(event `Dissolve`
  (bind _unitlocationbeforedissolve (`self.unitLocationBeforeDissolve`))
  ;[1 1 1] Moves the unit down below the ground over time when dead
  (set `self.unitLocationBeforeDissolve` (`self.K2_GetActorLocation`))
  (bind (_direction _alpha) (`Timeline|DissolveOverTime` :!via `PlayFromStart`)
    (:`Update`
      (`self.K2_SetActorLocation` (`KismetMathLibrary.VLerp` _unitlocationbeforedissolve (- _unitlocationbeforedissolve (0.0 0.0 200.0)) _alpha)))
    (:`Finished`
      (`self.K2_DestroyActor`))))

(fn `GetAnimation`
  (params (animationType :type "/Game/Match3RPGTemplate/Blueprints/Units/AnimationType Enum" :default "NewEnumerator0"))
  (returns (animation :type "AnimSequenceBase Object Reference") (isLoop :type Boolean))
  (return (select `/Game/Match3RPGTemplate/Blueprints/Units/AnimationType` animationType :`NewEnumerator0` (`self.idleAnimation`) :`NewEnumerator1` (`self.runAnimation`) :`NewEnumerator2` (`self.jumpBackAnimation`) :`NewEnumerator3` (`self.attackAnimation`) :`NewEnumerator7` (`self.GuardAnimation`) :`NewEnumerator4` (`self.getHitAnimation`) :`NewEnumerator5` (`self.dieAnimation`) :`NewEnumerator6` (`self.victoryAnimation`)) (select `/Game/Match3RPGTemplate/Blueprints/Units/AnimationType` animationType :`NewEnumerator0` true :`NewEnumerator1` true :`NewEnumerator2` true :`NewEnumerator6` true)))

(fn `IsUnitDead`
  (returns (isUnitDead :type Boolean))
  (return (<= (`self.currentHP`) 0)))

(fn `PlayAnimation`
  (params (animationType :type "/Game/Match3RPGTemplate/Blueprints/Units/AnimationType Enum" :default "NewEnumerator0"))
  (returns (animationLength :type "Float (double-precision)"))
  (bind (_animation _isloop) (`self.GetAnimation` animationType))
  (`SkeletalMeshComponent.PlayAnimation` (`self.SkeletalMesh`) _animation _isloop)
  (return (`AnimSequenceBase.SequenceLength` _animation)))

(fn `UserConstructionScript`)