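; BP_PlayerBase is the base player unit in the Match-3 RPG template, adding mana and armor-based health to its parent unit.
; On spawn, it adds the player controller's current armor HP to max HP, runs the parent spawn, then fills mana.
; Increase and reduce events route through SetMana, which clamps the value between zero and max and calls OnManaUpdated.
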(event `self.Spawn`
  (params (spawnLocation :type "/Game/Match3RPGTemplate/Blueprints/BP_UnitSpawnLocation Object Reference"))
  ;[1 1 1] Set mana when player unit is spawned
  (set `self.maxHP` (+ (`self.maxHP`) (`.HP_7_5FEEB6A04D020144057081887065E16D` (break `/Game/Match3RPGTemplate/Blueprints/Equipments/ArmorData` (`/Game/Match3RPGTemplate/Blueprints/BP_Match3RPGPlayerController.currentArmor` (cast `/Game/Match3RPGTemplate/Blueprints/BP_Match3RPGPlayerController` (`GameplayStatics.GetPlayerController` 0) :!pure true))))))
  (`parent.Spawn` spawnLocation)
  (`self.SetMana` (`self.maxMana`)))

(event `IncreaseMana`
  (params (mana :type Integer))
  ;[1 1 1] Increase mana
  (`self.SetMana` (+ mana (`self.currentMana`))))

(event `ReduceMana`
  (params (mana :type Integer))
  ;[1 1 1] Decrease mana
  (`self.SetMana` (- (`self.currentMana`) mana)))

(event `SetMana`
  (params (mana :type Integer))
  ;[1 1 1] Set mana
  (set `self.currentMana` (`KismetMathLibrary.Clamp` mana 0 (`self.maxMana`)))
  (`self.OnManaUpdated`))

(fn `UserConstructionScript`
  (`parent.UserConstructionScript`))