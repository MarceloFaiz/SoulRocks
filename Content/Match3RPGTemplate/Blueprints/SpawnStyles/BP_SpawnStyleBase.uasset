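; Base actor for unit spawn styles in a Match-3 RPG template, leaving the Spawn event empty for child classes to override.
; On BeginPlay it binds to its owning Unit's destroyed event and destroys itself along with that unit.
; HideUI and ShowUI helper events forward to the game UI on the Match-3 RPG player controller, when that UI is valid.
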(event `self.ReceiveBeginPlay`
  ;[1 1 1] Destroy when owning unit is destroyed
  (add `self.OnDestroyed` (`self.unit`) (delegate `OnUnitDestroyed`)))

(event `OnUnitDestroyed` :!signature `self.OnDestroyed`
  (params (DestroyedActor :type "Actor Object Reference"))
  ;[1 1 1] Destroy when owning unit is destroyed
  (`self.K2_DestroyActor`))

(event `Spawn`
  ;[1 1 1] Override in child class
)

(event `HideUI`
  ;[1 1 1] Hide / show UI
  (bind _asbp_match_3rpgplayer_controller (cast `/Game/Match3RPGTemplate/Blueprints/BP_Match3RPGPlayerController` (`GameplayStatics.GetPlayerController` 0)))
  (bind _gameui (`/Game/Match3RPGTemplate/Blueprints/BP_Match3RPGPlayerController.GameUI` _asbp_match_3rpgplayer_controller))
  (`/Engine/EditorBlueprintResources/StandardMacros.IsValid` _gameui
    (:`Is Valid`
      (`/Game/Match3RPGTemplate/Blueprints/UI/BP_GameUI.HideUI` _gameui))))

(event `ShowUI`
  ;[1 1 1] Hide / show UI
  (bind _asbp_match_3rpgplayer_controller (cast `/Game/Match3RPGTemplate/Blueprints/BP_Match3RPGPlayerController` (`GameplayStatics.GetPlayerController` 0)))
  (bind _gameui (`/Game/Match3RPGTemplate/Blueprints/BP_Match3RPGPlayerController.GameUI` _asbp_match_3rpgplayer_controller))
  (`/Engine/EditorBlueprintResources/StandardMacros.IsValid` _gameui
    (:`Is Valid`
      (`/Game/Match3RPGTemplate/Blueprints/UI/BP_GameUI.ShowUI` _gameui))))

(fn `UserConstructionScript`)