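; Spawn style for the Match3 RPG template that makes a unit run in from off screen to its spawn location.
; Spawn hides the UI and places the unit at an offset derived from the spawn point's forward vector.
; A timeline lerps the unit to the spawn point while an animation plays.
; On finish it switches animation, shows the UI and signals that spawning is done.
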(event `self.Spawn`
  (bind _spawnlocation (`self.spawnLocation`))
  (bind (_returnvalue_location _returnvalue_rotation _returnvalue_scale) (`KismetMathLibrary.BreakTransform` (`self.GetTransform` _spawnlocation)))
  ;[1 1 1] Run to spawn location from off screen
  (`self.HideUI`)
  (bind _output_get (set `self.startLocation` (+ _returnvalue_location (* (`self.GetActorForwardVector` _spawnlocation) (0.0 -750.0 0.0)))))
  (`self.K2_SetActorTransform` (`self.unit`) (`KismetMathLibrary.MakeTransform` _output_get _returnvalue_rotation _returnvalue_scale) false false)
  (`/Game/Match3RPGTemplate/Blueprints/Units/BP_UnitBase.PlayAnimation` (`self.unit`) "NewEnumerator1")
  (bind (_direction _alpha) (`Timeline|MoveOverTime` :!via `PlayFromStart`)
    (:`Update`
      (`self.K2_SetActorLocation` (`self.unit`) (`KismetMathLibrary.VLerp` (`self.startLocation`) (`self.K2_GetActorLocation` (`self.spawnLocation`)) _alpha) false false))
    (:`Finished`
      (`/Game/Match3RPGTemplate/Blueprints/Units/BP_UnitBase.PlayAnimation` (`self.unit`) "NewEnumerator0")
      (`self.ShowUI`)
      (`self.OnSpawnFinished`))))

(fn `UserConstructionScript`
  (`parent.UserConstructionScript`))