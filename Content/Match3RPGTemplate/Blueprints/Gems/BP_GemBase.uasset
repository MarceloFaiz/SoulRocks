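; BP_GemBase is the base gem Blueprint for the Match-3 RPG battle, with empty match and matching-details UI events for child gems to override.
; It destroys itself when its BattleManager is destroyed.
; Move helpers bind a callback to the manager's unit-moved event, then request a unit move.
; Player wrappers move the player to the current enemy's attack location, or back to spawn at double speed.
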(event `self.ReceiveBeginPlay`
  ;[1 1 1] Destroy when battle manager is destroyed
  (add `self.OnDestroyed` (`self.battleManager`) (delegate `OnBattleMangerDestroyed`)))

(event `OnBattleMangerDestroyed` :!signature `self.OnDestroyed`
  (params (DestroyedActor :type "Actor Object Reference"))
  ;[1 1 1] Destroy when battle manager is destroyed
  (`self.K2_DestroyActor`))

(event `UpdateMatchingDetails`
  (params (matchingDetailsUI :type "/Game/Match3RPGTemplate/Blueprints/UI/BP_MatchingDetailsUI Object Reference") (matchedGemAmount :type Integer))
  ;[1 1 1] Override in child class
)

(event `OnMatch`
  (params (matchedGemAmount :type Integer))
  ;[1 1 1] Override in child class
)

(fn `Move`
  (params (Move :type "Delegate (by ref)") (moveAnimation :type "/Game/Match3RPGTemplate/Blueprints/Units/AnimationType Enum" :default "NewEnumerator0") (moveSpeed :type "Float (double-precision)") (fromLocation :type "Vector Structure") (toLocation :type "Vector Structure") (unit :type "/Game/Match3RPGTemplate/Blueprints/Units/BP_UnitBase Object Reference"))
  (add `/Game/Match3RPGTemplate/Blueprints/BP_BattleManager.OnUnitMoved` (`self.battleManager`) Move)
  (`/Game/Match3RPGTemplate/Blueprints/BP_BattleManager.UnitMove` (`self.battleManager`) moveAnimation moveSpeed fromLocation toLocation unit))

(fn `PlayerMove`
  (params (PlayerMove :type "Delegate (by ref)"))
  (bind _battlemanager (`self.battleManager`))
  (bind _player (`/Game/Match3RPGTemplate/Blueprints/BP_BattleManager.player` _battlemanager))
  (`self.Move` PlayerMove "NewEnumerator1" (`/Game/Match3RPGTemplate/Blueprints/Units/BP_UnitBase.moveSpeed` _player) (`self.K2_GetActorLocation` _player) (`SceneComponent.K2_GetComponentLocation` (`/Game/Match3RPGTemplate/Blueprints/Units/BP_UnitBase.AttackLocation` (`/Game/Match3RPGTemplate/Blueprints/BP_BattleManager.currentEnemy` _battlemanager))) (`/Game/Match3RPGTemplate/Blueprints/BP_BattleManager.player` (`self.battleManager`))))

(fn `PlayerMoveBack`
  (params (PlayerMoveBack :type "Delegate (by ref)"))
  (bind _battlemanager (`self.battleManager`))
  (bind _player (`/Game/Match3RPGTemplate/Blueprints/BP_BattleManager.player` _battlemanager))
  (`self.Move` PlayerMoveBack "NewEnumerator2" (* (`/Game/Match3RPGTemplate/Blueprints/Units/BP_UnitBase.moveSpeed` _player) 2.0) (`self.K2_GetActorLocation` _player) (`SceneComponent.K2_GetComponentLocation` (`/Game/Match3RPGTemplate/Blueprints/Stages/BP_StageBase.PlayerSpawnLocation` (`/Game/Match3RPGTemplate/Blueprints/BP_BattleManager.stage` _battlemanager))) (`/Game/Match3RPGTemplate/Blueprints/BP_BattleManager.player` (`self.battleManager`))))

(fn `UserConstructionScript`)